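; BP_RangeHero_Child is a ranged hero child Blueprint that attacks by firing arrows at its target hero.
; ShootArrow triggers OnRangeAttackSpawn, which spawns a BP_Arrow at the mesh's arrow1Socket using the hero's rotation and scale.
; The arrow receives the hero as owner and parent and HeroToAttack as target, then runs SetupArrowInfo.
; BeginPlay, overlap and Tick are disabled stubs, and construction defers to the parent.
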(event Custom|OnRangeAttackSpawn
  (bind _returnvalue (Transformation|GetActorTransform))
  (bind _self self)
  (bind _returnvalue_2 (Game|SpawnActorfromClass "/Game/Gameplay/BP_Arrow.BP_Arrow_C" (Math|Transform|MakeTransform (Transformation|GetSocketLocation (Variables|Character|GetMesh) "arrow1Socket") (.rotation _returnvalue) (.scale _returnvalue)) "AlwaysSpawn" _self _self (Variables|Default|GetHero%20to%20Attack) _self))
  (Default|SetupArrowInfo _returnvalue_2))

(event EventBeginPlay
  (|CallParentFunction) ; This node is disabled and will not be called.\nDrag off pins to build functionality.
)

(event Collision|EventActorBeginOverlap
  (params (OtherActor :type Actor%20Object%20Reference))
  (|CallParentFunction OtherActor) ; This node is disabled and will not be called.\nDrag off pins to build functionality.
)

(event EventTick
  (params (DeltaSeconds :type Float%20%28single-precision%29))
  (|CallParentFunction DeltaSeconds) ; This node is disabled and will not be called.\nDrag off pins to build functionality.
)

(fn ConstructionScript
  (|CallParentFunction))

(fn ShootArrow
  (CallFunction|OnRangeAttackSpawn))