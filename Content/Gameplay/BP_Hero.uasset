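; Hero unit for a multiplayer, action-point game, with health, attacks and data-table-driven abilities.
; Tick walks it along a supplied path via AI MoveTo without pathfinding, and turns attacker or defender toward each other.
; Attack, hit, death and ability flags mark its state; hits spawn floating damage numbers, and death-animation completion destroys it.
; Separate client and server functions spawn spell actors after action-point and energy checks, with only the client displaying them on the grid.
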(event Custom|OnGetHit
  (bind _charachterstats (Variables|Default|GetCharachterStats))
  (bind _tempdamage (Variables|/Game/Core/CharcterComponents/BPC_CharachterStats.BPC_CharachterStats_C|GetTempDamage _charachterstats))
  ;[1 1 1] Always Called after the hit logic is excecuted
  (bind _currenthealth (Default|GetCurrentHealth (Variables|Default|GetCharachterStats)))
  (if (> _currenthealth 0)
    (Variables|Animation|SetIsHitted? true)
    (else
      (Variables|Animation|SetDead? true)))
  (if (!= _tempdamage 0)
    (Game|SpawnActorfromClass "/Game/Core/CharcterComponents/BP_FloatingNumber.BP_FloatingNumber_C" (Transformation|GetActorTransform) "Undefined" 0 _tempdamage 0)
    (Default|CallOnStatsChanged)))

(event Custom|OnHeroDie
  (Actor|DestroyActor))

(event EventBeginPlay
  (EventDispatchers|BindEventtoOnDeathAnimFinished (delegate Custom|OnHeroDie))
  (bind _spelldata (CallFunction|GetSpellDatafromDT (Variables|Ability|GetActiveAbility)))
  (Variables|Ability|SetAbilityCost (.Cost (Utilities|Struct|BreakS_Spell _spelldata))))

(event Collision|EventActorBeginOverlap
  (params (OtherActor :type Actor%20Object%20Reference)))

(event EventTick
  (params (DeltaSeconds :type Float%20%28single-precision%29))
  (bind _path (Variables|Default|Getpath))
  (bind _returnvalue (Utilities|Array|Length _path))
  (bind _returnvalue_2 (- _returnvalue 1))
  (CallFunction|RotateCharacterTowardEnemy)
  (if (and (!= _returnvalue 0) (!= _returnvalue_2 (Variables|Default|GetPathIndex)))
    (if (Math|Vector|Equal(Vector) (Math|Conversions|ToVector2D(Vector) (.location (Transformation|GetActorTransform))) (Math|Conversions|ToVector2D(Vector) (Utilities|Array|Get(acopy) (Variables|Default|Getpath) (Variables|Default|GetPathIndex))) 15.0)
      (bind _output_get (Variables|Default|SetPathIndex (+ (Variables|Default|GetPathIndex) 1)))
      (AI|Navigation|MovetoLocation (AI|GetAIController (Components|GetOwner)) (Utilities|Array|Get(acopy) (Variables|Default|Getpath) _output_get) 1e+01 false false false true 0 false))
    (elif (== _returnvalue_2 (Variables|Default|GetPathIndex))
      (if (Math|Vector|Equal(Vector) (Math|Conversions|ToVector2D(Vector) (.location (Transformation|GetActorTransform))) (Math|Conversions|ToVector2D(Vector) (Utilities|Array|Get(acopy) (Variables|Default|Getpath) (Variables|Default|GetPathIndex))) 15.0)
        (Default|CallOnMovementFinished)))))

(fn ConstructionScript)

(fn GetPlayerIndex
  (return (Variables|Default|GetPlayerIndex)))

(fn CreateandRunPath
  (params (path :type Array%20of%20Vectors))
  (bind _output_get (Variables|Default|Setpath path))
  (Variables|Default|SetPathIndex 0)
  (AI|Navigation|MovetoLocation (AI|GetAIController (Components|GetOwner)) (Utilities|Array|Get(acopy) _output_get) 1.0 false false false true 0 false))

(fn SetPlayerIndex
  (params (Index :type Integer))
  (Variables|Default|SetPlayerIndex Index))

(fn SetActionPoints
  (params (Points :type Integer))
  (if (Networking|IsServer)
    (Variables|Default|SetActionPoints Points)))

(fn GetActionPoints
  (return (Variables|Default|GetActionPoints)))

(fn AttackHero
  (params (HeroToAttack :type BP%20Hero%20Object%20Reference))
  (Variables|Default|SetHero%20to%20Attack HeroToAttack)
  (Variables|Default|SetRotateTowardEnemy? true))

(fn TriggerEnemyHitAnim
  (bind _hero_to_attack (Variables|Default|GetHero%20to%20Attack)
    (:then
      (CallFunction|OnGetHit _hero_to_attack)
      (Variables|Default|SetHero%20to%20Attack 0))
    (:else)))

(fn RotateCharacterTowardEnemy
  (bind _capsulecomponent (Variables|Collision|GetCapsuleComponent))
  (bind _capsulecomponent_2 (Variables|Collision|GetCapsuleComponent))
  (bind _returnvalue (Transformation|GetWorldLocation _capsulecomponent_2))
  (bind _returnvalue_2 (Transformation|GetWorldRotation _capsulecomponent_2))
  (bind _returnvalue_3 (Transformation|GetWorldLocation _capsulecomponent))
  (bind _returnvalue_4 (Transformation|GetWorldRotation _capsulecomponent))
  (if (Variables|Default|GetRotateTowardEnemy?)
    ;[1 1 1] Roatate When Attacking another Hero
    (bind _hero_to_attack (Variables|Default|GetHero%20to%20Attack)
      (:then
        (if (Math|Rotator|Equal(Rotator) (Math|Rotator|FindLookatRotation _returnvalue (+ (- (Transformation|GetWorldLocation (Variables|/Script/Engine.Character|GetCapsuleComponent _hero_to_attack)) (Transformation|GetWorldLocation (Variables|Collision|GetCapsuleComponent))) _returnvalue)) _returnvalue_2 1e+01)
          (Variables|Default|SetRotateTowardEnemy? false)
          (Variables|Animation|SetIsAttacking? true)
          (else
            (Transformation|SetActorRotation (Math|Interpolation|RInterpTo _returnvalue_2 (Math|Rotator|FindLookatRotation _returnvalue (+ (- (Transformation|GetWorldLocation (Variables|/Script/Engine.Character|GetCapsuleComponent _hero_to_attack)) (Transformation|GetWorldLocation (Variables|Collision|GetCapsuleComponent))) _returnvalue)) 0.5 0.7)))))
      (:else
        ;[1 1 1] Rotate When Hero Is going to be attacked
        (bind _attackinghero (Variables|Default|GetAttackingHero)
          (:then
            (if (Math|Rotator|Equal(Rotator) (Math|Rotator|FindLookatRotation _returnvalue_3 (+ (- (Transformation|GetWorldLocation (Variables|/Script/Engine.Character|GetCapsuleComponent _attackinghero)) (Transformation|GetWorldLocation (Variables|Collision|GetCapsuleComponent))) _returnvalue_3)) _returnvalue_4 1e+01)
              (Variables|Default|SetRotateTowardEnemy? false)
              (Variables|Default|SetAttackingHero 0)
              (else
                (Transformation|SetActorRotation (Math|Interpolation|RInterpTo _returnvalue_4 (Math|Rotator|FindLookatRotation _returnvalue_3 (+ (- (Transformation|GetWorldLocation (Variables|/Script/Engine.Character|GetCapsuleComponent _attackinghero)) (Transformation|GetWorldLocation (Variables|Collision|GetCapsuleComponent))) _returnvalue_3)) 0.5 0.7)))))
          (:else))))))

(fn PreparefortheHeroAttack
  (params (Attacking%20Hero :type BP%20Hero%20Object%20Reference))
  (Variables|Default|SetAttackingHero Attacking%20Hero)
  (Variables|Default|SetHero%20to%20Attack 0)
  (Variables|Default|SetRotateTowardEnemy? true))

(fn CreateHeroAbility-Client
  (params (Grid :type BP%20Grid%20Object%20Reference))
  (bind _self self)
  (if (> (Variables|Default|GetActionPoints) 0)
    (bind _spelldata (CallFunction|GetSpellDatafromDT (Variables|Ability|GetActiveAbility)))
    (if (<= (.Cost (Utilities|Struct|BreakS_Spell _spelldata)) (Variables|Ability|GetAbilityEnergy))
      (bind _returnvalue (Game|SpawnActorfromClass (.SpellClass (Utilities|Struct|BreakS_Spells_Assets (.Asset (Utilities|Struct|BreakS_Spell _spelldata)))) (Transformation|GetWorldTransform (Variables|Collision|GetCapsuleComponent)) "AlwaysSpawn" _self _self (.Range (Utilities|Struct|BreakS_Spell _spelldata)) 0))
      (Default|DisplayAbility _returnvalue (Transformation|GetActorLocation) Grid)
      (return _returnvalue))))

(fn IncreaseHeroAbilityEnergy
  (Variables|Ability|SetAbilityEnergy (+ (Variables|Ability|GetAbilityEnergy) 1)))

(fn CreateHeroAbility-Server
  (bind _self self)
  (if (> (Variables|Default|GetActionPoints) 0)
    (bind _spelldata (CallFunction|GetSpellDatafromDT (Variables|Ability|GetActiveAbility)))
    (if (<= (.Cost (Utilities|Struct|BreakS_Spell _spelldata)) (Variables|Ability|GetAbilityEnergy))
      (bind _returnvalue (Game|SpawnActorfromClass (.SpellClass (Utilities|Struct|BreakS_Spells_Assets (.Asset (Utilities|Struct|BreakS_Spell _spelldata)))) (Transformation|GetWorldTransform (Variables|Collision|GetCapsuleComponent)) "AlwaysSpawn" _self _self (.Range (Utilities|Struct|BreakS_Spell _spelldata)) 0))
      (return _returnvalue))))

(fn UseAbilty
  (Variables|Animation|SetIsAbility? true))