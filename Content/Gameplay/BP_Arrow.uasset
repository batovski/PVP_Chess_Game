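; BP_Arrow is a projectile actor that flies in a straight line toward a target hero.
; SetupArrowInfo computes a normalized direction toward TargetHero and rotates the arrow to face it.
; Tick moves the arrow with a swept step of FlyDirection times Speed per frame, without delta-time scaling.
; When its Box overlaps TargetHero, it calls TriggerEnemyHitAnim on ParentHero and destroys itself.
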(event OnComponentBeginOverlap(Box)
  (params (OverlappedComponent :type Primitive%20Component%20Object%20Reference) (OtherActor :type Actor%20Object%20Reference) (OtherComp :type Primitive%20Component%20Object%20Reference) (OtherBodyIndex :type Integer) (bFromSweep :type Boolean) (SweepResult :type Hit%20Result%20Structure%20%28by%20ref%29))
  (if (== OtherActor (Variables|Default|GetTargetHero))
    (Default|TriggerEnemyHitAnim (Variables|Default|GetParentHero))
    (Actor|DestroyActor)))

(event Collision|EventActorBeginOverlap
  (params (OtherActor :type Actor%20Object%20Reference)))

(event EventTick
  (params (DeltaSeconds :type Float%20%28single-precision%29))
  (Transformation|SetActorLocation self (+ (Transformation|GetActorLocation self) (* (Variables|Default|GetFly%20Direction) (Variables|Default|GetSpeed))) true false))

(fn ConstructionScript)

(fn SetupArrowInfo
  (Variables|Default|SetFly%20Direction (Math|Vector|Normalize (- (.location (Transformation|GetActorTransform (Variables|Default|GetTargetHero))) (.location (Transformation|GetActorTransform)))))
  (Transformation|SetActorRotation (Math|Rotator|FindLookatRotation (Transformation|GetActorLocation) (Transformation|GetActorLocation (Variables|Default|GetTargetHero))) true))