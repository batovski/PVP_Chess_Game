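; Player controller for a turn-based PvP grid game, handling turns, hero selection, movement and attacks.
; On its turn, clicks drive BP_Grid range previews and issue move, attack or move-then-attack server actions; Space ends the turn.
; Server actions check hero activity with the game mode and report completion through hero delegates.
; It also creates the HUD, relays match info through dispatchers and spawns character cards oriented per player.
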(event Custom|StartTurn_CLIENT
  (CallFunction|SetMyTurn true)
  (Default|UpdateOccupieData (Variables|Default|GetGrid) (Variables|Default|GetPlayer%20Index)))

(event Custom|EndTurn_CLIENT
  (CallFunction|SetMyTurn false))

(event Custom|Server%20Action%20-%20Move%20Hero
  (params (Hero :type BP%20Hero%20Object%20Reference) (Location :type Vector))
  (Variables|Default|SetIsPlayerControllerBusy? true)
  (Default|UnOccupieLocation (Variables|Default|GetGrid) (.location (Transformation|GetActorTransform Hero)))
  ;[1 1 1] Check if the Selected Hero Has Action Points Left
  (bind _asbpgm_turn_based_game_mode (Utilities|Casting|CastToBPGM_TurnBasedGameMode (Game|GetGameMode)))
  (bind _active_ (Default|IsHeroActive _asbpgm_turn_based_game_mode Hero))
  (if _active_
    (bind _returnvalue (Default|GetPathNodes (Variables|Default|GetGrid) (Transformation|GetActorLocation Hero) Location))
    (Default|CreateandRunPath Hero _returnvalue)
    (EventDispatchers|BindEventtoOnMovementFinished Hero (delegate Custom|OnCharacterMoveFinished))))

(event Custom|SetupPlayerOpponentRank
  (params (Rank :type Integer))
  (Default|CallOnPlayerOpponentRankChanged Rank))

(event Custom|OnOKButtonClicked
  (bind _asbp_pvpgame_instance (Utilities|Casting|CastToBP_PVPGameInstance (Game|GetGameInstance)))
  (Default|LeaveMatch _asbp_pvpgame_instance))

(event Custom|UpdateNewRankValue
  (params (New%20Rank :type Integer))
  (Default|CallOnPlayerNewRankChanged New%20Rank))

(event Custom|DisplayCharactersInfo
  (params (Team0 :type Array%20of%20BP%20Hero%20Object%20References) (Team1 :type Array%20of%20BP%20Hero%20Object%20References))
  (CallFunction|DisplayCharactersCards Team0 Team1))

(event Custom|OnCharacterAttackFinished
  (bind _asbpgm_turn_based_game_mode (Utilities|Casting|CastToBPGM_TurnBasedGameMode (Game|GetGameMode)))
  (Default|HeroAction _asbpgm_turn_based_game_mode (stale Custom|Server%20Action%20-%20Attack%20Hero SelectedHero))
  (EventDispatchers|UnbindEventfromOnAttackFinished (stale Custom|Server%20Action%20-%20Attack%20Hero SelectedHero) (delegate Custom|OnCharacterAttackFinished))
  (Variables|Default|SetIsPlayerControllerBusy? false))

(event Custom|EndMyTurn_SERVER
  (bind _asbpgm_turn_based_game_mode (Utilities|Casting|CastToBPGM_TurnBasedGameMode (Game|GetGameMode)))
  (Default|CycleTurns _asbpgm_turn_based_game_mode))

(event Custom|Server%20Action%20-%20Attack%20Hero
  (params (SelectedHero :type BP%20Hero%20Object%20Reference) (AttackedHero :type BP%20Hero%20Object%20Reference))
  (Variables|Default|SetIsPlayerControllerBusy? true)
  ;[1 1 1] Check for Action points
  (bind _asbpgm_turn_based_game_mode (Utilities|Casting|CastToBPGM_TurnBasedGameMode (Game|GetGameMode)))
  (bind _active_ (Default|IsHeroActive _asbpgm_turn_based_game_mode SelectedHero))
  (if _active_
    ;[1 1 1] Check for the actor position and decide can we attack him
    (Default|AttackHero SelectedHero AttackedHero)
    (bind _damage (Default|GetAttackDamage (Actor|GetComponentbyClass SelectedHero "/Game/Core/CharcterComponents/BPC_CharachterStats.BPC_CharachterStats_C")))
    (Default|PreparefortheHeroAttack AttackedHero SelectedHero)
    (Default|TakeDamage (Actor|GetComponentbyClass AttackedHero "/Game/Core/CharcterComponents/BPC_CharachterStats.BPC_CharachterStats_C") _damage)
    (EventDispatchers|BindEventtoOnAttackFinished SelectedHero (delegate Custom|OnCharacterAttackFinished))))

(event Custom|EndGame_CLIENT
  (params (Win? :type Boolean))
  (CallFunction|DisplayGameResults Win?))

(event Custom|SetPlayerIndex
  (params (PlayerIndex :type Integer))
  (Variables|Default|SetPlayer%20Index PlayerIndex))

(event Custom|OnCharacterMoveFinished
  (Default|OccupieLocation (Variables|Default|GetGrid) (stale Custom|Server%20Action%20-%20Move%20Hero Location))
  (bind _asbpgm_turn_based_game_mode (Utilities|Casting|CastToBPGM_TurnBasedGameMode (Game|GetGameMode)))
  (Default|HeroAction _asbpgm_turn_based_game_mode (stale Custom|Server%20Action%20-%20Move%20Hero Hero))
  (EventDispatchers|UnbindEventfromOnMovementFinished (stale Custom|Server%20Action%20-%20Move%20Hero Hero) (delegate Custom|OnCharacterMoveFinished))
  (Variables|Default|SetIsPlayerControllerBusy? false))

(event Custom|Server%20Action%20-%20Attack%20And%20Move
  (params (Selected%20Hero :type BP%20Hero%20Object%20Reference) (Attacked%20Hero :type BP%20Hero%20Object%20Reference) (Location :type Vector))
  (Variables|Default|SetIsPlayerControllerBusy? false)
  (Default|UnOccupieLocation (Variables|Default|GetGrid) (.location (Transformation|GetActorTransform)))
  ;[1 1 1] Check if the Selected Hero Has Action Points Left
  (bind _asbpgm_turn_based_game_mode (Utilities|Casting|CastToBPGM_TurnBasedGameMode (Game|GetGameMode)))
  (bind _active_ (Default|IsHeroActive _asbpgm_turn_based_game_mode Selected%20Hero))
  (if _active_
    (bind _returnvalue (Default|GetPathNodes (Variables|Default|GetGrid) (Transformation|GetActorLocation Selected%20Hero) Location))
    (Default|CreateandRunPath Selected%20Hero _returnvalue)
    (EventDispatchers|BindEventtoOnMovementFinished Selected%20Hero (delegate Custom|OnCharacterMoveFinishedAttack))))

(event Custom|OnCharacterMoveFinishedAttack
  (Default|OccupieLocation (Variables|Default|GetGrid) (stale Custom|Server%20Action%20-%20Attack%20And%20Move Location))
  (CallFunction|ServerAction-AttackHero (stale Custom|Server%20Action%20-%20Attack%20And%20Move Selected%20Hero) (stale Custom|Server%20Action%20-%20Attack%20And%20Move Attacked%20Hero))
  (EventDispatchers|UnbindEventfromOnMovementFinished (stale Custom|Server%20Action%20-%20Attack%20And%20Move Selected%20Hero) (delegate Custom|OnCharacterMoveFinishedAttack))
  (Variables|Default|SetIsPlayerControllerBusy? false))

(event Custom|SetPlayersInfo
  (params (PlayerName :type String) (OpponentName :type String))
  (Default|CallOnPlayersNameDisplayed PlayerName OpponentName)
  (Development|PrintString (Utilities|String|ToString(Integer) (Variables|Default|GetPlayer%20Index))))

(event EventBeginPlay
  ;[1 1 1] Find Grid in the Scene
  (bind _outactors (Actor|GetAllActorsOfClass "/Game/Core/BP_Grid.BP_Grid_C"))
  (Variables|Default|SetGrid (Utilities|Array|Get(acopy) _outactors))
  (if (Pawn|IsLocalController)
    (bind _returnvalue (UserInterface|CreateWidget "/Game/Interface/BPW_InGameHUD.BPW_InGameHUD_C" self))
    (UserInterface|Viewport|AddtoViewport _returnvalue 0)
    (EventDispatchers|BindEventtoOnOKButtonClicked _returnvalue (delegate Custom|OnOKButtonClicked))))

(event Input|MouseEvents|LeftMouseButton
  (params (Key :type Key%20Structure :default "None"))
  (:Pressed
    (if (Variables|Default|GetMyTurn)
      (CallFunction|HandleLeftMouse))))

(event Input|KeyboardEvents|SpaceBar
  (params (Key :type Key%20Structure :default "None"))
  (:Pressed
    (if (Variables|Default|GetMyTurn)
      (CallFunction|HandleEndTurn))))

(fn ConstructionScript)

(fn SetMyTurn
  (params (MyTurn :type Boolean))
  (bind _output_get (Variables|Default|SetMyTurn MyTurn))
  (Default|CallOnMyTurnChanged _output_get)
  (if (not _output_get)
    (Default|DeleteSelectedPath (Variables|Default|GetGrid))))

(fn HandleEndTurn
  (if (not (Variables|Default|GetIsPlayerControllerBusy?))
    (CallFunction|EndMyTurnSERVER)))

(fn HandleLeftMouse
  (bind (_hitresult _returnvalue) (Game|Player|GetHitResultUnderCursorbyChannel "TraceTypeQuery2" false))
  (bind _grid (Variables|Default|GetGrid))
  (bind _grid_2 (Variables|Default|GetGrid))
  (bind _grid_3 (Variables|Default|GetGrid))
  (bind _grid_4 (Variables|Default|GetGrid))
  (bind (_bblockinghit _binitialoverlap _time _distance _location _impactpoint _normal _impactnormal _physmat _hitactor) (Collision|BreakHitResult _hitresult))
  (if (not (Variables|Default|GetIsPlayerControllerBusy?))
    (Utilities|FlowControl|Sequence
      (:then_0
        (if _returnvalue
          ;[1 1 1] Set Proper New Location Based on the center of the cell
          (bind (_valid_ _rowx _columny) (Default|LocationtoTile _grid_3 _impactpoint))
          (if _valid_
            (bind _gridlocation (Default|TiletoGridLocation _grid_3 _rowx _columny true))
            (LocalVariables|SetNewlySelectedLocation (Math|Vector|MakeVector (.x _gridlocation) (.y _gridlocation) 0.0))
            (bind _asbp_hero (Utilities|Casting|CastToBP_Hero _hitactor))
            (bind _output_get (LocalVariables|SetNewlySelectedHero _asbp_hero))
            (bind _friendly_ (Utilities|IsFriendlyCharacter? _output_get))
            (if _friendly_
              (bind _actionpoints (Default|GetActionPoints _output_get))
              (if (> _actionpoints 0)
                (Default|CallOnSelected _output_get)
                (bind _movementpoints (Default|GetMovementRange (Actor|GetComponentbyClass _output_get "/Game/Core/CharcterComponents/BPC_CharachterStats.BPC_CharachterStats_C")))
                (Default|DisplayPossiblePaths (Variables|Default|GetGrid) _movementpoints (.location (Transformation|GetActorTransform _output_get)) (Variables|Default|GetPlayer%20Index)))))
          (else
            (return))))
      (:then_1
        (if (!= (Variables|Default|GetSelectedHero) (LocalVariables|GetNewlySelectedHero))
          (bind _newlyselectedhero (LocalVariables|GetNewlySelectedHero)
            (:then
              (bind _friendly__2 (Utilities|IsFriendlyCharacter? _newlyselectedhero))
              (if _friendly__2
                (bind _selectedhero (Variables|Default|GetSelectedHero)
                  (:then
                    (Default|CallOnUnSelected (Variables|Default|GetSelectedHero)))
                  (:else
                    _))
                (Variables|Default|SetSelectedHero (LocalVariables|GetNewlySelectedHero))
                (else
                  (Variables|Default|GetSelectedHero
                    (:then
                      ;[1 1 1] Display Attack Possibilities
                      (if (Variables|/Game/Core/BP_Grid.BP_Grid_C|GetIsDisplayed _grid)
                        (bind _attackrange (Default|GetAttackRange (Actor|GetComponentbyClass (Variables|Default|GetSelectedHero) "/Game/Core/CharcterComponents/BPC_CharachterStats.BPC_CharachterStats_C")))
                        (Default|DisplayAttackPath _grid _attackrange (LocalVariables|GetNewlySelectedLocation) (.location (Transformation|GetActorTransform (Variables|Default|GetSelectedHero))))
                        (Variables|Default|SetToAttackHero (LocalVariables|GetNewlySelectedHero))))
                    (:else)))))
            (:else
              (bind _selectedhero_2 (Variables|Default|GetSelectedHero)
                (:then
                  (bind _valid__2 (Default|VerifyDestination _grid_2 (LocalVariables|GetNewlySelectedLocation)))
                  (if _valid__2
                    (Default|OccupieLocation _grid_2 (LocalVariables|GetNewlySelectedLocation))
                    (Default|UnOccupieLocation _grid_2 (.location (Transformation|GetActorTransform (Variables|Default|GetSelectedHero))))
                    (bind _isattackpos_ (Default|IsAttackPosition _grid_2 (LocalVariables|GetNewlySelectedLocation)))
                    (if _isattackpos_
                      (CallFunction|ServerAction-AttackandMove (Variables|Default|GetSelectedHero) (Variables|Default|GetToAttackHero) (LocalVariables|GetNewlySelectedLocation))
                      (Variables|Default|SetToAttackHero 0 :!label _label)
                      (CallFunction|UnselectHero (Variables|Default|GetSelectedHero))
                      (else
                        (CallFunction|ServerAction-MoveHero (Variables|Default|GetSelectedHero) (LocalVariables|GetNewlySelectedLocation))
                        (CallFunction|UnselectHero (Variables|Default|GetSelectedHero))))
                    (Default|DeleteSelectedPath (Variables|Default|GetGrid) :!label _label_2)
                    (else
                      ;[1 1 1] Attack Without Moving
                      (bind (_valid__3 _rowx_2 _columny_2) (Default|LocationtoTile _grid_4 (.location (Transformation|GetActorTransform _selectedhero_2)) :!label _label_3))
                      (if _valid__3
                        (bind _gridlocation_2 (Default|TiletoGridLocation _grid_4 _rowx_2 _columny_2 true))
                        (if (Math|Vector|Equal(Vector) (LocalVariables|GetNewlySelectedLocation) (Math|Vector|MakeVector (.x _gridlocation_2) (.y _gridlocation_2) 0.0) 1.0)
                          (CallFunction|ServerAction-AttackHero (Variables|Default|GetSelectedHero) (Variables|Default|GetToAttackHero))
                          (goto _label)
                          (else
                            (Default|CallOnUnSelected (Variables|Default|GetSelectedHero))
                            (goto _label_2)))))))
                (:else))))
          (else
            (Variables|Default|GetToAttackHero
              (:then
                (goto _label_3))
              (:else))))))))

(fn GetGrid
  (return (Variables|Default|GetGrid)))

(fn DisplayGameResults
  (params (Win? :type Boolean))
  (Default|CallOnGameResultsDisplayed Win?))

(fn DisplayCharactersCards
  (params (Team0 :type Array%20of%20BP%20Hero%20Object%20References) (Team1 :type Array%20of%20BP%20Hero%20Object%20References))
  (bind _outactors (Actor|GetAllActorsOfClass "/Game/Core/SpawnSystem/BP_CharcterInfoSpawnPoint.BP_CharcterInfoSpawnPoint_C"))
  (for _array_element _outactors
    (if (== (Variables|/Game/Core/SpawnSystem/BP_CharcterInfoSpawnPoint.BP_CharcterInfoSpawnPoint_C|GetPlayerIndex _array_element) 0)
      (Utilities|Map|Add (LocalVariables|GetTeam%200%20Points) (Variables|/Game/Core/SpawnSystem/BP_CharcterInfoSpawnPoint.BP_CharcterInfoSpawnPoint_C|GetPointID _array_element) _array_element)
      (else
        (Utilities|Map|Add (LocalVariables|GetTeam%201%20Points) (Variables|/Game/Core/SpawnSystem/BP_CharcterInfoSpawnPoint.BP_CharcterInfoSpawnPoint_C|GetPointID _array_element) _array_element))))
  (bind _values (Utilities|Map|Values (LocalVariables|GetTeam%200%20Points)))
  (if (== 0 (Variables|Default|GetPlayer%20Index))
    (while (Math|Boolean|ANDBoolean (< (LocalVariables|GetPointIndex) (Utilities|Array|Length _values)) (< (LocalVariables|GetPointIndex) (Utilities|Array|Length Team0)) (< (LocalVariables|GetPointIndex) (Utilities|Array|Length Team1)))
      (bind _returnvalue (Game|SpawnActorfromClass "/Game/Core/MatchComponents/BP_CharcterCard.BP_CharcterCard_C" (Math|Transform|MakeTransform (.location (Transformation|GetActorTransform (.Value (Utilities|Map|Find (LocalVariables|GetTeam%200%20Points) (LocalVariables|GetPointIndex))))) (Math|Rotator|MakeRotator (.roll (.rotation (Transformation|GetActorTransform (.Value (Utilities|Map|Find (LocalVariables|GetTeam%200%20Points) (LocalVariables|GetPointIndex)))))) (.pitch (.rotation (Transformation|GetActorTransform (.Value (Utilities|Map|Find (LocalVariables|GetTeam%200%20Points) (LocalVariables|GetPointIndex)))))) (+ (.yaw (.rotation (Transformation|GetActorTransform (.Value (Utilities|Map|Find (LocalVariables|GetTeam%200%20Points) (LocalVariables|GetPointIndex)))))) -1.8e+02)) (.scale (Transformation|GetActorTransform (.Value (Utilities|Map|Find (LocalVariables|GetTeam%200%20Points) (LocalVariables|GetPointIndex)))))) "AlwaysSpawn" 0 0))
      (Default|SetupCharacterInfo _returnvalue (Utilities|Array|Get(acopy) Team0 (LocalVariables|GetPointIndex)))
      (bind _returnvalue_2 (Game|SpawnActorfromClass "/Game/Core/MatchComponents/BP_CharcterCard.BP_CharcterCard_C" (Math|Transform|MakeTransform (.location (Transformation|GetActorTransform (.Value (Utilities|Map|Find (LocalVariables|GetTeam%201%20Points) (LocalVariables|GetPointIndex))))) (Math|Rotator|MakeRotator (.roll (.rotation (Transformation|GetActorTransform (.Value (Utilities|Map|Find (LocalVariables|GetTeam%201%20Points) (LocalVariables|GetPointIndex)))))) (.pitch (.rotation (Transformation|GetActorTransform (.Value (Utilities|Map|Find (LocalVariables|GetTeam%201%20Points) (LocalVariables|GetPointIndex)))))) (+ (.yaw (.rotation (Transformation|GetActorTransform (.Value (Utilities|Map|Find (LocalVariables|GetTeam%201%20Points) (LocalVariables|GetPointIndex)))))) -1.8e+02)) (.scale (Transformation|GetActorTransform (.Value (Utilities|Map|Find (LocalVariables|GetTeam%201%20Points) (LocalVariables|GetPointIndex)))))) "AlwaysSpawn" 0 0))
      (Default|SetupCharacterInfo _returnvalue_2 (Utilities|Array|Get(acopy) Team1 (LocalVariables|GetPointIndex)))
      (LocalVariables|SetPointIndex (+ (LocalVariables|GetPointIndex) 1)))
    (else
      (LocalVariables|SetPointIndex 1)
      (while (Math|Boolean|ANDBoolean (<= (LocalVariables|GetPointIndex) (Utilities|Array|Length _values)) (<= (LocalVariables|GetPointIndex) (Utilities|Array|Length Team0)) (<= (LocalVariables|GetPointIndex) (Utilities|Array|Length Team1)))
        (bind _values_2 (Utilities|Map|Values (LocalVariables|GetTeam%201%20Points)))
        (bind _returnvalue_3 (Game|SpawnActorfromClass "/Game/Core/MatchComponents/BP_CharcterCard.BP_CharcterCard_C" (Transformation|GetActorTransform (.Value (Utilities|Map|Find (LocalVariables|GetTeam%201%20Points) (- (Utilities|Array|Length _values_2) (LocalVariables|GetPointIndex))))) "AlwaysSpawn" 0 0))
        (Default|SetupCharacterInfo _returnvalue_3 (Utilities|Array|Get(acopy) Team1 (- (LocalVariables|GetPointIndex) 1)))
        (bind _values_3 (Utilities|Map|Values (LocalVariables|GetTeam%200%20Points)))
        (bind _returnvalue_4 (Game|SpawnActorfromClass "/Game/Core/MatchComponents/BP_CharcterCard.BP_CharcterCard_C" (Transformation|GetActorTransform (.Value (Utilities|Map|Find (LocalVariables|GetTeam%200%20Points) (- (Utilities|Array|Length _values_3) (LocalVariables|GetPointIndex))))) "AlwaysSpawn" 0 0))
        (Default|SetupCharacterInfo _returnvalue_4 (Utilities|Array|Get(acopy) Team0 (- (LocalVariables|GetPointIndex) 1)))
        (LocalVariables|SetPointIndex (+ (LocalVariables|GetPointIndex) 1))))))

(fn UnselectHero
  (params (Hero :type BP%20Hero%20Object%20Reference))
  (Default|CallOnUnSelected Hero)
  (Variables|Default|SetSelectedHero Hero))