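; BP_TurnBasePlayerState is a player state that carries each player's PlayFab ID and display name in a turn-based PVP game.
; On BeginPlay, only remote (non-authority) instances read both values from BP_PVPGameInstance and send them to the server through two setter events.
; Those ServerSet events simply store the values on the player state, and Tick is unused.
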(event Custom|ServerSetPlayerID
  (params (PlayFabID :type String))
  (Variables|Default|SetPlayFabID PlayFabID))

(event Custom|ServerSetPlayerName
  (params (PlayerName :type String))
  (Variables|Default|SetPlayerName PlayerName))

(event EventBeginPlay
  (Networking|SwitchHasAuthority
    (:Remote
      (bind _asbp_pvpgame_instance (Utilities|Casting|CastToBP_PVPGameInstance (Game|GetGameInstance)))
      (CallFunction|ServerSetPlayerID (Variables|/Game/Core/BP_PVPGameInstance.BP_PVPGameInstance_C|GetPlayFabID _asbp_pvpgame_instance))
      (CallFunction|ServerSetPlayerName (Variables|/Game/Core/BP_PVPGameInstance.BP_PVPGameInstance_C|GetPlayerName _asbp_pvpgame_instance)))))

(event EventTick
  (params (DeltaSeconds :type Float%20%28single-precision%29)))

(fn ConstructionScript)