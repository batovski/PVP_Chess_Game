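; BP_Grid is the tile board for hero tactics, handling tile/location conversion, path queries and move/attack highlights.
; Construction lays out tiles as instanced meshes; BeginPlay builds GridData, blocking obstacle tiles found by box overlap and occupying hero tiles.
; GridData supplies paths and reachable tiles, while multicast events update occupancy.
; Maps of highlighted tiles validate clicks, and attack previews sink overlapping move instances below the board until cleared.
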(event Custom|Multicast%20-%20Occupie%20Location
  (params (Location :type Vector))
  (Public|OccupieLocation Location))

(event Custom|Multicast%20-%20Unoccupie%20Location
  (params (Location :type Vector))
  (Public|UnOccupieLocation Location))

(event EventBeginPlay
  (Class|GridDataComponent|CreateGrid (Variables|Default|GetGridData) (Variables|Constants|GetNumColoms) (Variables|Constants|GetNumRows))
  (Public|FindObsticales)
  (Private|FindHerosStartPos))

(event Collision|EventActorBeginOverlap
  (params (OtherActor :type Actor%20Object%20Reference)))

(event EventTick
  (params (DeltaSeconds :type Float%20%28single-precision%29)))

(fn ConstructionScript
  (bind _returnvalue (Transformation|GetActorTransform))
  (for _index (range 0 (- (Variables|Constants|GetNumRows) 1))
    (for _index_2 (range 0 (- (Variables|Constants|GetNumColoms) 1))
      (bind (_valid_ _grid_location_x _grid_location_y) (Public|TiletoGridLocalLocation _index _index_2 true))
      (Components|InstancedStaticMesh|AddInstance (Variables|Default|GetGridInstancedMesh) (Math|Transform|MakeTransform (Math|Vector|MakeVector _grid_location_x _grid_location_y (.z (.location _returnvalue))) (.rotation _returnvalue) (.scale _returnvalue))))))

(fn LocationtoTile
  (params (Location :type Vector))
  (bind _returnvalue (Transformation|GetActorLocation))
  (bind _returnvalue_2 (Transformation|GetActorLocation))
  (bind _tilesize (Variables|Constants|GetTileSize))
  (bind _tilesize_2 (Variables|Constants|GetTileSize))
  (bind _returnvalue_3 (- (.y Location) (.y _returnvalue)))
  (bind _returnvalue_4 (- (.x Location) (.x _returnvalue_2)))
  (bind _returnvalue_5 (/ _returnvalue_4 _tilesize_2))
  (bind _returnvalue_6 (/ _returnvalue_3 _tilesize))
  (bind _returnvalue_7 (Math|Float|Floor _returnvalue_5))
  (bind _returnvalue_8 (Math|Float|Floor _returnvalue_6))
  (bind _valid_ (Utilities|TileValid _returnvalue_7 _returnvalue_8))
  (return _valid_ _returnvalue_7 _returnvalue_8))

(fn TiletoGridLocation
  (params (Row :type Integer) (Column :type Integer) (Center? :type Boolean))
  (bind _returnvalue (Transformation|GetActorLocation))
  (bind _tilesize (Variables|Constants|GetTileSize))
  (bind _returnvalue_2 (/ _tilesize 2.0))
  (bind _returnvalue_3 (select Center? _returnvalue_2 0.0))
  (bind _valid_ (Utilities|TileValid Row Column))
  (return _valid_ (Math|Vector2D|MakeVector2D (+ (+ (* Row (Variables|Constants|GetTileSize)) (.x _returnvalue)) _returnvalue_3) (+ (+ (.y _returnvalue) (* Column (Variables|Constants|GetTileSize))) _returnvalue_3))))

(fn DeleteSelectedPath
  (Components|InstancedStaticMesh|ClearInstances (Variables|Default|GetMoveGridInstancedMesh))
  (Utilities|Map|Clear (Variables|Default|GetPossibleMovePath))
  (Components|InstancedStaticMesh|ClearInstances (Variables|Default|GetAttackInstancedMesh))
  (Utilities|Map|Clear (Variables|Default|GetPossibleAttackPath))
  (Variables|Default|SetIsDisplayed false))

(fn GetPossibleMoves
  (params (StartPos :type Vector) (NumberOfSteps :type Integer))
  (bind (_valid_ _rowx _columny) (public|LocationtoTile StartPos))
  (LocalVariables|SetRowX _rowx)
  (LocalVariables|SetColumnY _columny)
  (if _valid_
    (for _index (range 1 NumberOfSteps)
      (Utilities|FlowControl|Sequence
        (:then_0
          ;[1 1 1] -1,0
          (bind (_valid__2 _gridlocation) (Public|TiletoGridLocation (- (LocalVariables|GetRowX) _index) (LocalVariables|GetColumnY) false))
          (if _valid__2
            (Utilities|Array|Add (LocalVariables|GetGrid) _gridlocation)))
        (:then_1
          ;[1 1 1] -1,1
          (bind (_valid__3 _gridlocation_2) (Public|TiletoGridLocation (- (LocalVariables|GetRowX) _index) (+ (LocalVariables|GetColumnY) _index) false))
          (if _valid__3
            (Utilities|Array|Add (LocalVariables|GetGrid) _gridlocation_2)))
        (:then_2
          ;[1 1 1] 0,1
          (bind (_valid__4 _gridlocation_3) (Public|TiletoGridLocation (LocalVariables|GetRowX) (+ (LocalVariables|GetColumnY) _index) false))
          (if _valid__4
            (Utilities|Array|Add (LocalVariables|GetGrid) _gridlocation_3)))
        (:then_3
          ;[1 1 1] 1,1
          (bind (_valid__5 _gridlocation_4) (Public|TiletoGridLocation (+ (LocalVariables|GetRowX) _index) (+ (LocalVariables|GetColumnY) _index) false))
          (if _valid__5
            (Utilities|Array|Add (LocalVariables|GetGrid) _gridlocation_4)))
        (:then_4
          ;[1 1 1] 0,1
          (bind (_valid__6 _gridlocation_5) (Public|TiletoGridLocation (+ (LocalVariables|GetRowX) _index) (LocalVariables|GetColumnY) false))
          (if _valid__6
            (Utilities|Array|Add (LocalVariables|GetGrid) _gridlocation_5)))
        (:then_5
          ;[1 1 1] 1,-1
          (bind (_valid__7 _gridlocation_6) (Public|TiletoGridLocation (+ (LocalVariables|GetRowX) _index) (- (LocalVariables|GetColumnY) _index) false))
          (if _valid__7
            (Utilities|Array|Add (LocalVariables|GetGrid) _gridlocation_6)))
        (:then_6
          ;[1 1 1] 0,-1
          (bind (_valid__8 _gridlocation_7) (Public|TiletoGridLocation (LocalVariables|GetRowX) (- (LocalVariables|GetColumnY) _index) false))
          (if _valid__8
            (Utilities|Array|Add (LocalVariables|GetGrid) _gridlocation_7)))
        (:then_7
          ;[1 1 1] -1,-1
          (bind (_valid__9 _gridlocation_8) (Public|TiletoGridLocation (- (LocalVariables|GetRowX) _index) (- (LocalVariables|GetColumnY) _index) false))
          (if _valid__9
            (Utilities|Array|Add (LocalVariables|GetGrid) _gridlocation_8)))
        (:then_8
          (return (LocalVariables|GetGrid)))))))

(fn VerifyDestination
  (params (Destination :type Vector))
  (bind _possiblemovepath (Variables|Default|GetPossibleMovePath))
  (bind (_valid_ _rowx _columny) (public|LocationtoTile Destination))
  (bind (_valid__2 _grid_location_x _grid_location_y) (Public|TiletoGridLocalLocation _rowx _columny true))
  (if _valid__2
    (Utilities|Map|Keys _possiblemovepath)
    (if (Utilities|Map|Contains _possiblemovepath (Math|Vector2D|MakeVector2D _grid_location_x _grid_location_y))
      (return true)
      (else
        _)))
  (return false))

(fn DisplayPossiblePaths
  (params (ActionPoints :type Integer) (Position :type Vector) (Player%20Index :type Integer))
  (bind _returnvalue (Transformation|GetActorTransform))
  (bind _returnvalue_2 (Transformation|GetActorTransform))
  (bind _tilesize (Variables|Constants|GetTileSize))
  (bind _returnvalue_3 (/ _tilesize 2.0))
  (bind (_valid_ _rowx _columny) (public|LocationtoTile Position))
  (if _valid_
    (Components|InstancedStaticMesh|ClearInstances (Variables|Default|GetMoveGridInstancedMesh))
    (Components|InstancedStaticMesh|ClearInstances (Variables|Default|GetMoveGridInstancedMesh))
    (Components|InstancedStaticMesh|ClearInstances (Variables|Default|GetAttackInstancedMesh))
    (Utilities|Map|Clear (Variables|Default|GetPossibleMovePath))
    (Utilities|Map|Clear (Variables|Default|GetPossibleAttackPath))
    (Variables|Default|SetIsDisplayed true)
    (bind _returnvalue_4 (Class|GridDataComponent|GetPossiblePaths (Variables|Default|GetGridData) _rowx _columny ActionPoints))
    (for _array_element _returnvalue_4
      (if (.isoccupied _array_element)
        (bind _gridlocation (Public|TiletoGridLocation (.x _array_element) (.y _array_element) true))
        (bind _outactors (Collision|BoxOverlapActors (Math|Vector|MakeVector (.x _gridlocation) (.y _gridlocation) 0.0) (Math|Vector|MakeVector _returnvalue_3 _returnvalue_3 1e+01) (LocalVariables|GetNewLocalVar_0) "/Game/Gameplay/BP_Hero.BP_Hero_C" (LocalVariables|GetNewLocalVar_1) :!class /Script/Engine.KismetSystemLibrary))
        (for _array_element_2 _outactors
          (bind _asbp_hero (Utilities|Casting|CastToBP_Hero _array_element_2))
          (bind _playerindex (Default|GetPlayerIndex _asbp_hero))
          (if (!= Player%20Index _playerindex)
            (bind (_valid__2 _grid_location_x _grid_location_y) (Public|TiletoGridLocalLocation (.x _array_element) (.y _array_element) true))
            (Components|InstancedStaticMesh|AddInstance (Variables|Default|GetAttackInstancedMesh) (Math|Transform|MakeTransform (Math|Vector|MakeVector _grid_location_x _grid_location_y (.z (.location _returnvalue_2))) (.rotation _returnvalue_2) (.scale _returnvalue_2)))))
        (else
          (bind (_valid__3 _grid_location_x_2 _grid_location_y_2) (Public|TiletoGridLocalLocation (.x _array_element) (.y _array_element) true))
          (bind _returnvalue_5 (Components|InstancedStaticMesh|AddInstance (Variables|Default|GetMoveGridInstancedMesh) (Math|Transform|MakeTransform (Math|Vector|MakeVector _grid_location_x_2 _grid_location_y_2 0.0) (.rotation _returnvalue) (.scale _returnvalue))))
          (Utilities|Map|Add (Variables|Default|GetPossibleMovePath) (Math|Vector2D|MakeVector2D _grid_location_x_2 _grid_location_y_2) _returnvalue_5))))))

(fn FindObsticales
  (bind _tilesize (Variables|Constants|GetTileSize))
  (bind _returnvalue (/ _tilesize 2.0))
  (for _index (range 0 (- (Variables|Constants|GetNumRows) 1))
    (for _index_2 (range 0 (- (Variables|Constants|GetNumColoms) 1))
      (bind (_valid_ _gridlocation) (Public|TiletoGridLocation _index _index_2 true))
      (if _valid_
        (bind _returnvalue_2 (Collision|BoxOverlapActors (Math|Vector|MakeVector (.x _gridlocation) (.y _gridlocation) (.z (.location (Transformation|GetActorTransform)))) (Math|Vector|MakeVector _returnvalue _returnvalue 5.0) (LocalVariables|Gettype) "/Game/Core/BP_Obstical.BP_Obstical_C" (LocalVariables|GetIgnore) :!class /Script/Engine.KismetSystemLibrary))
        (if _returnvalue_2
          (Class|GridDataComponent|BlockNode (Variables|Default|GetGridData) _index _index_2))))))

(fn GetPathNodes
  (params (StartPos :type Vector) (Dest :type Vector))
  (bind _path (LocalVariables|GetPath))
  (bind (_valid_ _rowx _columny) (public|LocationtoTile StartPos))
  (if _valid_
    (bind (_valid__2 _rowx_2 _columny_2) (public|LocationtoTile Dest))
    (if _valid__2
      (bind _returnvalue (Class|GridDataComponent|GetPath (Variables|Default|GetGridData) _rowx _columny _rowx_2 _columny_2))
      (for _array_element _returnvalue
        (bind (_valid__3 _gridlocation) (Public|TiletoGridLocation (.x _array_element) (.y _array_element) true))
        (if _valid__3
          (Utilities|Array|Add _path (Math|Conversions|ToVector(Vector2D) _gridlocation (.z Dest)))))
      (return _path))))

(fn TiletoGridLocalLocation
  (params (Row :type Integer) (Column :type Integer) (Center? :type Boolean))
  (bind _tilesize (Variables|Constants|GetTileSize))
  (bind _returnvalue (/ _tilesize 2.0))
  (bind _returnvalue_2 (select Center? _returnvalue 0.0))
  (bind _valid_ (Utilities|TileValid Row Column))
  (return _valid_ (+ (* Row (Variables|Constants|GetTileSize)) _returnvalue_2) (+ (* Column (Variables|Constants|GetTileSize)) _returnvalue_2)))

(fn OccupieLocation
  (params (Location :type Vector))
  (bind (_valid_ _rowx _columny) (public|LocationtoTile Location))
  (if _valid_
    (Class|GridDataComponent|OccupieNode (Variables|Default|GetGridData) _rowx _columny)))

(fn UnOccupieLocation
  (params (Location :type Vector))
  (bind (_valid_ _rowx _columny) (public|LocationtoTile Location))
  (if _valid_
    (Class|GridDataComponent|UnOccupieNode (Variables|Default|GetGridData) _rowx _columny)))

(fn UpdateOccupieData
  (params (CurrentPlayerIndex :type Integer))
  (bind _tilesize (Variables|Constants|GetTileSize))
  (bind _griddata (Variables|Default|GetGridData))
  (bind _returnvalue (/ _tilesize 2.0))
  (for _index (range 0 (- (Variables|Constants|GetNumRows) 1))
    (for _index_2 (range 0 (- (Variables|Constants|GetNumColoms) 1))
      (bind _gridlocation (Public|TiletoGridLocation _index _index_2 true))
      (bind _outactors (Collision|BoxOverlapActors (Math|Vector|MakeVector (.x _gridlocation) (.y _gridlocation) (.z (.location (Transformation|GetActorTransform)))) (Math|Vector|MakeVector _returnvalue _returnvalue 4e+01) (LocalVariables|GetNewLocalVar_3) "/Game/Gameplay/BP_Hero.BP_Hero_C" (LocalVariables|GetNewLocalVar_2) :!class /Script/Engine.KismetSystemLibrary))
      (for _array_element _outactors
        (Utilities|Casting|CastToBP_Hero _array_element
          (:then
            (Class|GridDataComponent|OccupieNode _griddata _index _index_2))
          (:CastFailed
            (Class|GridDataComponent|UnOccupieNode _griddata _index _index_2)))))))

(fn DisplayAttackPath
  (params (AttackDistance :type Integer) (Position :type Vector) (HeroPosition :type Vector))
  (bind _returnvalue (Transformation|GetActorTransform))
  (bind (_valid_ _rowx _columny) (public|LocationtoTile Position))
  (if _valid_
    (bind (_valid__2 _rowx_2 _columny_2) (public|LocationtoTile HeroPosition))
    (Private|ClearAttackPath)
    (Utilities|Map|Clear (Variables|Default|GetPossibleAttackPath))
    (Components|InstancedStaticMesh|ClearInstances (Variables|Default|GetAttackInstancedMesh))
    (bind _returnvalue_2 (Class|GridDataComponent|GetPossiblePaths (Variables|Default|GetGridData) _rowx _columny AttackDistance))
    (for _array_element _returnvalue_2
      (bind (_valid__3 _grid_location_x _grid_location_y) (Public|TiletoGridLocalLocation (.x _array_element) (.y _array_element) true))
      (if (.ReturnValue (Utilities|Map|Find (Variables|Default|GetPossibleMovePath) (Math|Vector2D|MakeVector2D _grid_location_x _grid_location_y)))
        (Components|InstancedStaticMesh|AddInstance (Variables|Default|GetAttackInstancedMesh) (Math|Transform|MakeTransform (Math|Vector|MakeVector _grid_location_x _grid_location_y (.z (.location _returnvalue))) (.rotation _returnvalue) (.scale _returnvalue)) :!label _label)
        (Utilities|Map|Add (Variables|Default|GetPossibleAttackPath) (Math|Vector2D|MakeVector2D _grid_location_x _grid_location_y) (.Value (Utilities|Map|Find (Variables|Default|GetPossibleMovePath) (Math|Vector2D|MakeVector2D _grid_location_x _grid_location_y))))
        (Components|InstancedStaticMesh|UpdateInstanceTransform (Variables|Default|GetMoveGridInstancedMesh) (.Value (Utilities|Map|Find (Variables|Default|GetPossibleMovePath) (Math|Vector2D|MakeVector2D _grid_location_x _grid_location_y))) (Math|Transform|MakeTransform (Math|Vector|MakeVector _grid_location_x _grid_location_y -2e+02) (.rotation _returnvalue) (.scale _returnvalue)) false true false)
        (else
          (bind (_valid__4 _grid_location_x_2 _grid_location_y_2) (Public|TiletoGridLocalLocation _rowx_2 _columny_2 true))
          (if (and (== _grid_location_x_2 _grid_location_x) (== _grid_location_y_2 _grid_location_y))
            (goto _label)))))))

(fn ClearAttackPath
  (bind _returnvalue (Transformation|GetActorTransform))
  (bind _movegridinstancedmesh (Variables|Default|GetMoveGridInstancedMesh))
  (bind _values (Utilities|Map|Values (Variables|Default|GetPossibleAttackPath)))
  (for _array_element _values
    (Components|InstancedStaticMesh|UpdateInstanceTransform _movegridinstancedmesh _array_element (Math|Transform|MakeTransform (Math|Vector|MakeVector (.x (.location (.OutInstanceTransform (Components|InstancedStaticMesh|GetInstanceTransform _movegridinstancedmesh _array_element false)))) (.y (.location (.OutInstanceTransform (Components|InstancedStaticMesh|GetInstanceTransform _movegridinstancedmesh _array_element false)))) (.z (.location _returnvalue))) (.rotation _returnvalue) (.scale _returnvalue)) false true true)))

(fn IsAttackPosition
  (params (Position :type Vector))
  (bind (_valid_ _rowx _columny) (public|LocationtoTile Position))
  (bind (_valid__2 _grid_location_x _grid_location_y) (Public|TiletoGridLocalLocation _rowx _columny true))
  (return (Utilities|Map|Contains (Variables|Default|GetPossibleAttackPath) (Math|Vector2D|MakeVector2D _grid_location_x _grid_location_y))))

(fn FindHerosStartPos
  (bind _outactors (Actor|GetAllActorsOfClass "/Game/Gameplay/BP_Hero.BP_Hero_C"))
  (for _array_element _outactors
    (Public|OccupieLocation (Transformation|GetActorLocation _array_element))))