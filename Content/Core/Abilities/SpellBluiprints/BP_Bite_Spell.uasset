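; BP_Bite_Spell is a Bite spell ability that applies an effect to the selected hero.
; Its Use Ability override runs the parent logic, then looks up the data table entry for its Effect.
; It adds that entry's effect Blueprint to the EffectContainer on the target's BPC_CharachterStats component.
; The event graph holds only disabled default events.
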(event EventBeginPlay
  (|CallParentFunction) ; This node is disabled and will not be called.\nDrag off pins to build functionality.
)

(event Collision|EventActorBeginOverlap
  (params (OtherActor :type Actor%20Object%20Reference))
  (|CallParentFunction OtherActor) ; This node is disabled and will not be called.\nDrag off pins to build functionality.
)

(event EventTick
  (params (DeltaSeconds :type Float%20%28single-precision%29))
  (|CallParentFunction DeltaSeconds) ; This node is disabled and will not be called.\nDrag off pins to build functionality.
)

(fn ConstructionScript
  (|CallParentFunction))

(fn UseAbility
  (params (Parent%20Hero :type BP%20Hero%20Object%20Reference) (Selected%20Hero :type BP%20Hero%20Object%20Reference))
  ;[1 1 1] Ecxecute Logic
  (|CallParentFunction Parent%20Hero Selected%20Hero)
  (bind _effectdata (CallFunction|GetEffectDatafromDT (Variables|Default|GetEffect)))
  (Default|AddEffect (Variables|/Game/Core/CharcterComponents/BPC_CharachterStats.BPC_CharachterStats_C|GetEffectContainer (Actor|GetComponentbyClass Selected%20Hero "/Game/Core/CharcterComponents/BPC_CharachterStats.BPC_CharachterStats_C")) (.BP_Effect (Utilities|Struct|BreakS_Effect_Assets (.Assets (Utilities|Struct|BreakS_Effect_Data _effectdata))))))