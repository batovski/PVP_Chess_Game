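; BP_TurnBasedPawn is the pawn for a turn-based grid game that keeps the grid's selected tile under the mouse cursor.
; Every tick it gets the grid from BP_TurnBasedPlayerController and runs a complex Visibility trace under the cursor.
; A hit location is converted to row and column and set as the selected tile, while a miss sets an invalid tile index.
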(event EventBeginPlay)

(event Collision|EventActorBeginOverlap
  (params (OtherActor :type Actor%20Object%20Reference)))

(event EventTick
  (params (DeltaSeconds :type Float%20%28single-precision%29))
  (CallFunction|UpdateCursorPosition))

(fn ConstructionScript)

(fn UpdateCursorPosition
  (bind _returnvalue (Game|GetPlayerController 0))
  (bind (_hitresult _returnvalue_2) (Game|Player|GetHitResultUnderCursorbyChannel _returnvalue "TraceTypeQuery1" true))
  (bind _asbp_turn_based_player_controller (Utilities|Casting|CastToBP_TurnBasedPlayerController (Game|GetPlayerController 0)))
  (bind _grid (Default|GetGrid _asbp_turn_based_player_controller))
  (LocalVariables|SetGrid _grid)
  (if _returnvalue_2
    (bind _output_get (LocalVariables|SetHitLocation (.Location (Collision|BreakHitResult _hitresult))))
    (bind (_valid_ _rowx _columny) (Default|LocationtoTile (LocalVariables|GetGrid) _output_get))
    (Default|SetSelectedTile (LocalVariables|GetGrid) _rowx _columny)
    (else
      (Default|SetSelectedTile (LocalVariables|GetGrid) -1 -1))))