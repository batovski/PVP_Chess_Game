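; BPC_CharachterStats is an actor component holding a character's health, speed, attack and attack range for the turn-based game.
; TakeDamage lowers Health and, at zero, casts the owner to BP_Hero, notifies BPGM_TurnBasedGameMode through HeroDies, then destroys the owner.
; Simple getters expose movement range, attack damage and attack range.
; The move and attack validity checks are stubs that always return true, leaving a distance check unused.
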(event EventBeginPlay)

(event EventTick
  (params (DeltaSeconds :type Float%20%28single-precision%29)))

(fn TakeDamage
  (params (Damage :type Integer))
  (bind _output_get (Variables|CharacterStats|SetHealth (- (Variables|CharacterStats|GetHealth) Damage)))
  (Development|PrintString (Utilities|String|ToString(Integer) _output_get))
  (if (<= _output_get 0)
    (bind _asbpgm_turn_based_game_mode (Utilities|Casting|CastToBPGM_TurnBasedGameMode (Game|GetGameMode)))
    (bind _asbp_hero (Utilities|Casting|CastToBP_Hero (Components|GetOwner)))
    (Default|HeroDies _asbpgm_turn_based_game_mode _asbp_hero)
    (CallFunction|Die)))

(fn GetMovementRange
  (return (Variables|CharacterStats|GetSpeed)))

(fn GetAttackDamage
  (return (Variables|CharacterStats|GetAttack)))

(fn Die
  (Development|PrintString "Death")
  (Actor|DestroyActor (Components|GetOwner)))

(fn IsAttackPossible
  (params (NewParam :type Vector))
  (return true))

(fn IsMovePossible
  (params (Destination :type Vector))
  (return true))

(fn GetAttackRange
  (return (Variables|CharacterStats|GetAttackRange)))