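; Hero component that holds timed status effects, each represented by a spawned effect actor.
; AddEffect spawns the effect class at the hero with a duration and image, stores it and signals a stats change.
; TickEffectsUpdate, not driven by Tick, applies each effect, decrements and multicasts its duration, then removes and destroys expired ones mid-loop.
; A separate multicast relays stat-change notifications to the hero.
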(event Custom|Add%20Effect
  (params (New%20effect :type BP%20Effect%20Base%20Class%20Reference) (Duration :type Integer) (Image :type Texture%202D%20Object%20Reference))
  (CallFunction|AddEffect New%20effect Duration Image))

(event Custom|Update%20Effects%20-%20MULTICAST
  (params (NewDuration :type Integer) (Effect :type BP%20Effect%20Base%20Object%20Reference))
  (Default|CallOnEffectChanged NewDuration Effect))

(event Custom|Update%20Charatcer%20Stats%20Data%20-%20MULTICAST
  (bind _asbp_hero (Utilities|Casting|CastToBP_Hero (Components|GetOwner)))
  (Default|CallOnStatsChanged _asbp_hero))

(event EventBeginPlay
  (bind _asbp_hero (Utilities|Casting|CastToBP_Hero (Components|GetOwner)))
  (Variables|Default|SetOwnerHero _asbp_hero))

(event EventTick
  (params (DeltaSeconds :type Float%20%28single-precision%29)))

(fn TickEffectsUpdate
  (for _array_element (Variables|Default|GetEffects)
    (Default|ApplyEffect _array_element (Variables|Default|GetOwnerHero))
    (bind _output_get (Variables|/Game/Core/Effects/BP_Effects/BP_EffectBase.BP_EffectBase_C|SetEffectDuration _array_element (- (Variables|/Game/Core/Effects/BP_Effects/BP_EffectBase.BP_EffectBase_C|GetEffectDuration _array_element) 1)))
    (CallFunction|UpdateEffects-MULTICAST _output_get _array_element)
    (if (<= (Variables|/Game/Core/Effects/BP_Effects/BP_EffectBase.BP_EffectBase_C|GetEffectDuration _array_element) 0)
      (LocalVariables|SetTempActor _array_element)
      (Utilities|Array|RemoveItem (Variables|Default|GetEffects) _array_element)
      (bind _tempactor (LocalVariables|GetTempActor)
        (:then
          (Actor|DestroyActor _tempactor))
        (:else)))))

(fn AddEffect
  (params (New%20effect :type BP%20Effect%20Base%20Class%20Reference) (Duration :type Integer) (Image :type Texture%202D%20Object%20Reference))
  (bind _returnvalue (Components|GetOwner))
  (bind _returnvalue_2 (Game|SpawnActorfromClass New%20effect (Transformation|GetActorTransform _returnvalue) "AlwaysSpawn" _returnvalue Duration Image 0))
  (Utilities|Array|AddUnique (Variables|Default|GetEffects) _returnvalue_2)
  (bind _asbp_hero (Utilities|Casting|CastToBP_Hero _returnvalue))
  (Default|CallOnStatsChanged _asbp_hero))