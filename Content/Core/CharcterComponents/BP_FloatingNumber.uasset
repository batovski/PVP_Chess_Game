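; BP_FloatingNumber is an actor that shows a floating number through a widget component, then removes itself.
; On BeginPlay it casts the widget to BPW_FloatingPoints, passes it the Number variable through OnNumberSpawnEvent and prints that value.
; It binds to the end of the widget's HUDFloatingNumberAnim and destroys itself when that fires, so the animation sets its lifetime.
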(event Custom|OnAnimationFinished
  (Actor|DestroyActor))

(event EventBeginPlay
  (bind _number (Variables|Default|GetNumber))
  (bind _asbpw_floating_points (Utilities|Casting|CastToBPW_FloatingPoints (UserInterface|GetUserWidgetObject (Variables|Default|GetWidget))))
  (Class|UserWidget|BindtoAnimationFinished _asbpw_floating_points (Variables|/Game/Interface/BPW_FloatingPoints.BPW_FloatingPoints_C|GetHUD_FloatingNumberAnim _asbpw_floating_points) (delegate Custom|OnAnimationFinished))
  (Default|OnNumberSpawnEvent _asbpw_floating_points _number)
  (Development|PrintString (Utilities|String|ToString(Integer) _number)))

(event Collision|EventActorBeginOverlap
  (params (OtherActor :type Actor%20Object%20Reference)))

(event EventTick
  (params (DeltaSeconds :type Float%20%28single-precision%29)))

(fn ConstructionScript)