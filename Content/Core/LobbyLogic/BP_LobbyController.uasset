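; BP_LobbyController is the lobby player controller that connects the lobby HUD to online login and matchmaking.
; On BeginPlay it creates the BPW_LobbyHUD widget, adds it to the viewport, casts the game instance to BP_PVPGameInstance and binds the HUD's button events.
; The login button calls ConnectToPlayfab and the battle button calls FindMatch, both on the game instance.
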(event Custom|OnBattleBTN_click
  (Default|FindMatch (stale EventBeginPlay _asbp_pvpgame_instance)))

(event Custom|OnLoginBTN_click
  (Default|ConnecttoPlayfab (stale EventBeginPlay _asbp_pvpgame_instance)))

(event EventBeginPlay
  (bind _returnvalue (UserInterface|CreateWidget "/Game/Interface/BPW_LobbyHUD.BPW_LobbyHUD_C" self))
  (UserInterface|Viewport|AddtoViewport _returnvalue 0)
  (bind _asbp_pvpgame_instance (Utilities|Casting|CastToBP_PVPGameInstance (Game|GetGameInstance)))
  (EventDispatchers|BindEventtoOnLoginClicked _returnvalue (delegate Custom|OnLoginBTN_click))
  (EventDispatchers|BindEventtoOnBattleBTNClick _returnvalue (delegate Custom|OnBattleBTN_click)))

(event EventTick
  (params (DeltaSeconds :type Float%20%28single-precision%29)))

(fn ConstructionScript)