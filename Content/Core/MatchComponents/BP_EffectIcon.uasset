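; BP_EffectIcon is a match actor that displays an effect as an icon with its remaining duration as text.
; On BeginPlay it creates a dynamic instance of MI_Image for the Icon, sets its Image as the texture and writes the starting duration to DurationTXT.
; UpdateData stores and displays a new duration, destroying the actor and returning true once it reaches zero or below.
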(event EventBeginPlay
  (bind _returnvalue (Rendering|Material|CreateDynamicMaterialInstance "/Game/Meshes/Cards/MI_Image.MI_Image" "None" "None" :!class /Script/Engine.KismetMaterialLibrary))
  (Rendering|Material|SetMaterial (Variables|Default|GetIcon) 0 _returnvalue)
  (Rendering|Material|SetTextureParameterValue _returnvalue "Texture" (Variables|Default|GetImage))
  (Rendering|Components|TextRender|SetText (Variables|Default|GetDurationTXT) (Utilities|Text|ToText(Integer) (Variables|Default|GetEffectDuration))))

(event Collision|EventActorBeginOverlap
  (params (OtherActor :type Actor%20Object%20Reference)))

(event EventTick
  (params (DeltaSeconds :type Float%20%28single-precision%29)))

(fn ConstructionScript)

(fn UpdateData
  (params (Duration :type Integer))
  (bind _output_get (Variables|Default|SetEffectDuration Duration))
  (Rendering|Components|TextRender|SetText (Variables|Default|GetDurationTXT) (Utilities|Text|ToText(Integer) _output_get))
  (if (<= _output_get 0)
    (Actor|DestroyActor)
    (return true)
    (else
      (return false))))