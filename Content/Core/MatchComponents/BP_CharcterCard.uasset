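; BP_CharcterCard is a 3D card actor showing a match character's name, avatar, stats, skill icon and team-colored front.
; SetupCharacterInfo fills it through dynamic materials and binds to character events; stat refreshes show a skull at zero health.
; CardFlyUp raises and tilts it toward the player, CardLand restores it, and clicking Plane2 while raised displays the ability grid once.
; Effect icons are spawned attached, tracked in a map, and re-spaced upon removal.
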(event OnClicked(Plane2)
  (params (TouchedComponent :type Primitive%20Component%20Object%20Reference) (ButtonPressed :type Key%20Structure :default "None"))
  (if (Variables|Default|GetSelected?)
    (if (not (Variables|Default|GetSpellClicked))
      (Variables|Default|GetCharacter
        (:then
          (Default|DisplayAbilityGridData (Variables|Default|GetPlayerController) (Variables|Default|GetCharacter))
          (Variables|Default|SetSpellClicked true))
        (:else)))))

(event EventBeginPlay
  (Variables|Default|SetStartLocation (Transformation|GetActorLocation))
  (Variables|Default|SetStartRotation (Transformation|GetActorRotation)))

(event Collision|EventActorBeginOverlap
  (params (OtherActor :type Actor%20Object%20Reference)))

(event EventTick
  (params (DeltaSeconds :type Float%20%28single-precision%29)))

(event EventDestroyed)

(fn ConstructionScript)

(fn SetupCharacterInfo
  (params (Character :type BP%20Hero%20Object%20Reference) (Friendly? :type Boolean))
  (bind _returnvalue (Actor|GetComponentbyClass Character "/Game/Core/CharcterComponents/BPC_CharachterStats.BPC_CharachterStats_C"))
  (Variables|Default|SetCharacter Character)
  (EventDispatchers|BindEventtoOnStatsChanged Character (EventDispatchers|CreateEvent :!event OnStatChnaged))
  (bind _currenthealth (Default|GetCurrentHealth _returnvalue))
  (Rendering|Components|TextRender|SetText (Variables|Default|GetHealthPoints) (Utilities|Text|ToText(Integer) _currenthealth))
  (Rendering|Components|TextRender|SetText (Variables|Default|GetNameRender) (Utilities|Text|ToText(String) (Variables|/Game/Gameplay/BP_Hero.BP_Hero_C|GetHeroName Character)))
  (bind _movementpoints (Default|GetMovementRange _returnvalue))
  (Rendering|Components|TextRender|SetText (Variables|Default|GetMovePoints) (Utilities|Text|ToText(Integer) _movementpoints))
  (bind _damage (Default|GetAttackDamage _returnvalue))
  (Rendering|Components|TextRender|SetText (Variables|Default|GetDamagePoints) (Utilities|Text|ToText(Integer) _damage))
  (EventDispatchers|BindEventtoOnSelected (Variables|Default|GetCharacter) (EventDispatchers|CreateEvent :!event CardFlyUp))
  (EventDispatchers|BindEventtoOnUnSelected (Variables|Default|GetCharacter) (EventDispatchers|CreateEvent :!event CardLand))
  (EventDispatchers|BindEventtoOnEffectChanged (Variables|/Game/Gameplay/BP_Hero.BP_Hero_C|GetEffectContainer (Variables|Default|GetCharacter)) (EventDispatchers|CreateEvent :!event UpdateEffectsIconsData))
  (bind _spelldata (CallFunction|GetSpellDatafromDT (Variables|/Game/Gameplay/BP_Hero.BP_Hero_C|GetActiveAbility Character)))
  (bind _returnvalue_2 (Rendering|Material|CreateDynamicMaterialInstance "/Game/Meshes/Cards/MI_Image.MI_Image" "None" "None" :!class /Script/Engine.KismetMaterialLibrary))
  (Rendering|Material|SetMaterial (Variables|Default|GetSkillIcon) 0 _returnvalue_2)
  (Rendering|Material|SetTextureParameterValue _returnvalue_2 "Texture" (.Icon (Utilities|Struct|BreakS_Spells_Assets (.Asset (Utilities|Struct|BreakS_Spell _spelldata)))))
  (bind _returnvalue_3 (Rendering|Material|CreateDynamicMaterialInstance "/Game/Meshes/Cards/MI_Image.MI_Image" "None" "None" :!class /Script/Engine.KismetMaterialLibrary))
  (Rendering|Material|SetMaterial (Variables|Default|GetAvatar) 0 _returnvalue_3)
  (Rendering|Material|SetTextureParameterValue _returnvalue_3 "Texture" (Variables|/Game/Gameplay/BP_Hero.BP_Hero_C|GetHeroAvatar Character))
  (if Friendly?
    (bind _returnvalue_4 (Rendering|Material|CreateDynamicMaterialInstance "/Game/Meshes/Cards/MI_Card_Front.MI_Card_Front" "None" "None" :!class /Script/Engine.KismetMaterialLibrary))
    (bind _output_get (LocalVariables|SetMaterial _returnvalue_4))
    (Rendering|Material|SetMaterial (Variables|Default|GetCardMesh) 0 _output_get)
    (Rendering|Material|SetTextureParameterValue (LocalVariables|GetMaterial) "Texture" "/Game/Meshes/Cards/Textures/silver_blue_front.silver_blue_front")
    (else
      (bind _returnvalue_5 (Rendering|Material|CreateDynamicMaterialInstance "/Game/Meshes/Cards/MI_Card_Front.MI_Card_Front" "None" "None" :!class /Script/Engine.KismetMaterialLibrary))
      (bind _output_get_2 (LocalVariables|SetMaterial _returnvalue_5))
      (Rendering|Material|SetMaterial (Variables|Default|GetCardMesh) 0 _output_get_2)
      (Rendering|Material|SetTextureParameterValue (LocalVariables|GetMaterial) "Texture" "/Game/Meshes/Cards/Textures/silver_red_front.silver_red_front"))))

(fn CardFlyUp
  (bind _returnvalue (Transformation|GetActorLocation))
  (bind _returnvalue_2 (Transformation|GetActorLocation))
  (bind _returnvalue_3 (Game|Player|GetPlayerPawn 0))
  (bind _returnvalue_4 (Transformation|GetActorLocation _returnvalue_3))
  (bind _returnvalue_5 (Transformation|GetActorLocation _returnvalue_3))
  (bind _returnvalue_6 (- _returnvalue_5 _returnvalue_2))
  (bind _returnvalue_7 (Math|Rotator|FindLookatRotation _returnvalue _returnvalue_4))
  (Variables|Default|GetCharacter
    (:then
      (if (not (Variables|Default|GetSelected?))
        (Transformation|SetActorLocation (+ (Transformation|GetActorLocation) (Math|Vector|MakeVector (* (.x _returnvalue_6) 0.1) (* (.y _returnvalue_6) 0.3) 2.5e+02)) true false)
        (Transformation|SetActorRotation (Math|Rotator|MakeRotator (.roll _returnvalue_7) (.pitch _returnvalue_7) (.yaw (Transformation|GetActorRotation))))
        (Variables|Default|SetSelected? true)))
    (:else)))

(fn CardLand
  (if (not (not (Variables|Default|GetSelected?)))
    (Transformation|SetActorLocation (Variables|Default|GetStartLocation) true false)
    (Transformation|SetActorRotation (Variables|Default|GetStartRotation))
    (Variables|Default|SetSelected? false)
    (Variables|Default|SetSpellClicked false)))

(fn OnStatChnaged
  (bind _character (Variables|Default|GetCharacter))
  (bind _effectsicons (Variables|Default|GetEffectsIcons))
  (bind _returnvalue (Actor|GetComponentbyClass _character "/Game/Core/CharcterComponents/BPC_CharachterStats.BPC_CharachterStats_C"))
  (Variables|Default|GetCharacter
    (:then
      (bind _currenthealth (Default|GetCurrentHealth _returnvalue))
      (Rendering|Components|TextRender|SetText (Variables|Default|GetHealthPoints) (Utilities|Text|ToText(Integer) _currenthealth))
      (if (== _currenthealth 0)
        (bind _returnvalue_2 (Rendering|Material|CreateDynamicMaterialInstance "/Game/Meshes/Cards/MI_Image.MI_Image" "None" "None" :!class /Script/Engine.KismetMaterialLibrary))
        (Rendering|Material|SetMaterial (Variables|Default|GetAvatar) 0 _returnvalue_2)
        (Rendering|Material|SetTextureParameterValue _returnvalue_2 "Texture" "/Game/Assets/GUI/skull_01.skull_01"))
      (bind _movementpoints (Default|GetMovementRange _returnvalue))
      (Rendering|Components|TextRender|SetText (Variables|Default|GetMovePoints) (Utilities|Text|ToText(Integer) _movementpoints))
      (bind _damage (Default|GetAttackDamage _returnvalue))
      (Rendering|Components|TextRender|SetText (Variables|Default|GetDamagePoints) (Utilities|Text|ToText(Integer) _damage))
      (for (_array_element _array_index) (Variables|/Game/Core/CharcterComponents/BPC_EffectContainer.BPC_EffectContainer_C|GetEffects (Variables|/Game/Gameplay/BP_Hero.BP_Hero_C|GetEffectContainer (Variables|Default|GetCharacter)))
        ;[1 1 1] Effect Icon Display
        (if (Utilities|Map|Contains _effectsicons _array_element)
          (Default|UpdateData (.Value (Utilities|Map|Find _effectsicons _array_element)) (Variables|/Game/Core/Effects/BP_Effects/BP_EffectBase.BP_EffectBase_C|GetEffectDuration _array_element))
          (else
            (bind _returnvalue_3 (Game|SpawnActorfromClass "/Game/Core/MatchComponents/BP_EffectIcon.BP_EffectIcon_C" (Math|Transform|MakeTransform (+ (.location (Transformation|GetWorldTransform (Variables|Default|GetEffects%20Start%20Position))) (Math|Vector|MakeVector (* (* _array_index (Math|Float|Truncate (Variables|Default|GetIconGap))) (.x (Math|Vector|Normalize (- (Transformation|GetActorLocation (Game|Player|GetPlayerPawn 0)) (Transformation|GetActorLocation))))) 0.0 0.0) "") (Transformation|GetWorldRotation (Variables|Default|GetCardMesh)) "1,1,1") "AlwaysSpawn" self (Variables|/Game/Core/Effects/BP_Effects/BP_EffectBase.BP_EffectBase_C|GetEffectDuration _array_element) "NewEnumerator0" (Variables|/Game/Core/Effects/BP_Effects/BP_EffectBase.BP_EffectBase_C|GetImage _array_element) 0))
            (Transformation|AttachActorToActor _returnvalue_3 self "None" "KeepWorld" "KeepWorld" "KeepWorld" true)
            (Utilities|Map|Add _effectsicons _array_element _returnvalue_3)))))
    (:else)))

(fn UpdateEffectsIconsData
  (params (NewDuration :type Integer) (Effect :type BP%20Effect%20Base%20Object%20Reference))
  (bind _effectsicons (Variables|Default|GetEffectsIcons))
  (bind (_value _returnvalue) (Utilities|Map|Find _effectsicons Effect))
  (if _returnvalue
    (bind _destroyed_ (Default|UpdateData _value NewDuration))
    (if _destroyed_
      (Utilities|Map|Remove (Variables|Default|GetEffectsIcons) Effect)
      (bind _values (Utilities|Map|Values (Variables|Default|GetEffectsIcons)))
      (for (_array_element _array_index) _values
        (Transformation|SetWorldLocation (Variables|/Game/Core/MatchComponents/BP_EffectIcon.BP_EffectIcon_C|GetDefaultSceneRoot _array_element) (+ (.location (Transformation|GetWorldTransform (Variables|Default|GetEffects%20Start%20Position))) (Math|Vector|MakeVector (* (* _array_index (Math|Float|Truncate (Variables|Default|GetIconGap))) (.x (Math|Vector|Normalize (- (Transformation|GetActorLocation (Game|Player|GetPlayerPawn 0)) (Transformation|GetActorLocation))))) 0.0 0.0) "") false false)))))