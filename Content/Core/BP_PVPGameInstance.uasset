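; Game instance for PVP matchmaking, combining PlayFab Multiplayer with Steam login and Advanced Sessions.
; Account info supplies the title player ID for a PVP_QUEUE ticket, which a looping timer polls until matched.
; The member loop branches on team: Team 1 creates a session tagged with the MatchId, while Team 2 waits, searches by that ID and joins.
; Failures print through a shared handler; the queue statistics success handler is empty.
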(event Custom|Connect%20to%20playfab
  (bind _authtoken (Class|AdvancedIdentityLibrary|GetPlayerAuthToken (Game|GetPlayerController 0))
    (:OnSuccess
      (|LoginwithSteam (Utilities|Struct|MakeClientLoginWithSteamRequest true 0 "" 0 "" _authtoken) (delegate Custom|Success%20Connect) (delegate Custom|Failed%20Connect)))
    (:OnFailure
      (Development|PrintString "FAILED TO GET TOKEN"))))

(event Custom|Success%20Connect
  (params (result :type Client%20Login%20Result%20Structure) (customData :type Object%20Object%20Reference))
  (Development|PrintString "Successful Connected")
  (Variables|Default|SetPlayFabID (.PlayFabId (Utilities|Struct|BreakClientLoginResult result))))

(event Custom|SuccessGetTicket
  (params (result :type Multiplayer%20Get%20Matchmaking%20Ticket%20Result%20Structure) (customData :type Object%20Object%20Reference))
  (bind (_cancellationreasonstring _changenumber _created _creator _giveupafterseconds _matchid _members _memberstomatchwith _queuename _status) (Utilities|Struct|BreakMultiplayerGetMatchmakingTicketResult result))
  (if (Utilities|Enum|Equal(Enum) _status "Matched")
    (Utilities|Time|ClearandInvalidateTimerbyHandle (Variables|Default|GetSearchingTimerHandler))
    (CallFunction|GetMatch _matchid _queuename)))

(event Custom|FailedGetTicket
  (params (error :type Play%20Fab%20Error%20Structure) (customData :type Object%20Object%20Reference))
  (CallFunction|Failed error))

(event Custom|GetMatch
  (params (MatchId :type String) (Queue%20Name :type String))
  (|GetMatch (Utilities|Struct|MakeMultiplayerGetMatchRequest 0 false MatchId Queue%20Name) (delegate Custom|SuccessGetMatch) (delegate Custom|FailedGetMatch)))

(event Custom|FailedGetMatch
  (params (error :type Play%20Fab%20Error%20Structure) (customData :type Object%20Object%20Reference))
  (CallFunction|Failed error))

(event Custom|SuccessGetMatch
  (params (result :type Multiplayer%20Get%20Match%20Result%20Structure) (customData :type Object%20Object%20Reference))
  (bind (_arrangementstring _matchid _members) (Utilities|Struct|BreakMultiplayerGetMatchResult result))
  (for _array_element _members
    (switch string (Class|PlayFabJsonObject|GetStringField _array_element)
      (:team1
        (|AdvancedSession (Utilities|Array|MakeArray (Class|AdvancedSessionsLibrary|MakeLiteralSessionPropertyString "MatchId" _matchid)) 0 100 0 false true false true true true false false false true false true))
      (:team2
        (Utilities|FlowControl|Delay 5.0)
        (bind _results (|FindSessionsAdvanced 0 0 false "AllServers" (Utilities|Array|MakeArray (Class|AdvancedSessionsLibrary|MakeLiteralSessionSearchProperty (Class|AdvancedSessionsLibrary|MakeLiteralSessionPropertyString "MatchId" _matchid) "Equals")) false false false true)
          (:OnSuccess
            (|JoinSession 0 (Utilities|Array|Get(acopy) _results))))))))

(event Custom|GetQueueStatistics
  (params (Queue :type String))
  (|GetQueueStatistics (Utilities|Struct|MakeMultiplayerGetQueueStatisticsRequest 0 Queue) (delegate Custom|SuccessQueueStats) (delegate Custom|FailedGetQueueStatistics)))

(event Custom|FailedGetQueueStatistics
  (params (error :type Play%20Fab%20Error%20Structure) (customData :type Object%20Object%20Reference))
  (CallFunction|Failed error))

(event Custom|SuccessQueueStats
  (params (result :type Multiplayer%20Get%20Queue%20Statistics%20Result%20Structure) (customData :type Object%20Object%20Reference)))

(event Custom|FailedGetAccountInfo
  (params (error :type Play%20Fab%20Error%20Structure) (customData :type Object%20Object%20Reference))
  (CallFunction|Failed error))

(event Custom|Failed%20Connect
  (params (error :type Play%20Fab%20Error%20Structure) (customData :type Object%20Object%20Reference))
  (CallFunction|Failed error))

(event Custom|GetAccountInfo
  (|GetAccountInfo (Utilities|Struct|MakeClientGetAccountInfoRequest "" (Variables|Default|GetPlayFabID)) (delegate Custom|SuccessAccountInfo) (delegate Custom|FailedGetAccountInfo)))

(event Custom|SuccessAccountInfo
  (params (result :type Client%20Get%20Account%20Info%20Result%20Structure) (customData :type Object%20Object%20Reference))
  (Utilities|FlowControl|Sequence
    (:then_1
      (CallFunction|CreatematchMakingTicket (Class|PlayFabJsonObject|GetStringField (Class|PlayFabJsonObject|GetObjectField (Class|PlayFabJsonObject|GetObjectField (.AccountInfo (Utilities|Struct|BreakClientGetAccountInfoResult result)) "TitleInfo") "TitlePlayerAccount") "Id") "PVP_QUEUE"))))

(event Custom|CreateMatchMakingTicket
  (params (Player%20Id :type String) (Queue%20Name :type String))
  (Development|PrintString Player%20Id)
  (Development|PrintString Queue%20Name)
  (|DestroySession (Game|GetPlayerController 0)
    (:then
      (Variables|Default|SetCreatorSettings (Class|PlayFabJsonObject|ConstructJsonObject))
      (Variables|Default|SetEntityKeySettings (Class|PlayFabJsonObject|ConstructJsonObject))
      (Class|PlayFabJsonObject|SetStringField (Variables|Default|GetEntityKeySettings) "Id" Player%20Id)
      (Class|PlayFabJsonObject|SetStringField (Variables|Default|GetEntityKeySettings) "Type" "title_player_account")
      (Class|PlayFabJsonObject|SetStringField (Variables|Default|GetEntityKeySettings) "TypeString" "title_player_account")
      (Class|PlayFabJsonObject|SetObjectField (Variables|Default|GetCreatorSettings) "Entity" (Variables|Default|GetEntityKeySettings))
      (|MatchmakingTicket (Utilities|Struct|MakeMultiplayerCreateMatchmakingTicketRequest (Variables|Default|GetCreatorSettings) 0 120 (Utilities|Array|MakeArray 0) Queue%20Name) (delegate Custom|SuccessCreateMatchMaking) (delegate Custom|FailedMatchMaking)))))

(event Custom|FailedMatchMaking
  (params (error :type Play%20Fab%20Error%20Structure) (customData :type Object%20Object%20Reference))
  (CallFunction|Failed error))

(event Custom|SuccessCreateMatchMaking
  (params (result :type Multiplayer%20Create%20Matchmaking%20Ticket%20Result%20Structure) (customData :type Object%20Object%20Reference))
  (Variables|Default|SetTicket%20Id (.TicketId (Utilities|Struct|BreakMultiplayerCreateMatchmakingTicketResult result)))
  (bind _returnvalue (Utilities|Time|SetTimerbyFunctionName 0 "CheckIfMatchFound" 1e+01 true))
  (Variables|Default|SetSearchingTimerHandler _returnvalue))

(event Custom|GetMatchMakingTicket
  (params (QueueName :type String) (TicketId :type String))
  (|GetMatchmakingTicket (Utilities|Struct|MakeMultiplayerGetMatchmakingTicketRequest 0 false QueueName TicketId) (delegate Custom|SuccessGetTicket) (delegate Custom|FailedGetTicket)))

(fn Failed
  (params (Errors :type Play%20Fab%20Error%20Structure))
  (bind (_haserror _errorcode _errorname _errormessage _errordetails) (Utilities|Struct|BreakPlayFabError Errors))
  (Development|PrintString _errorname)
  (Development|PrintString _errormessage)
  (Development|PrintString _errordetails))

(fn CheckifMatchFound
  (CallFunction|GetMatchMakingTicket "PVP_QUEUE" (Variables|Default|GetTicket%20Id)))