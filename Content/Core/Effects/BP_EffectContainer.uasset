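; Effect container that holds the active effect actors for its owning hero.
; AddEffect registers effects uniquely, and TickEffectsUpdate applies each one to OwnerHero, then removes and destroys any whose duration has run out.
; Event Tick is unused, so updates depend on external calls to TickEffectsUpdate.
; Removal happens inside the loop over the same array, which can skip the following effect.
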(event EventBeginPlay)

(event EventTick
  (params (DeltaSeconds :type Float%20%28single-precision%29)))

(fn TickEffectsUpdate
  (for _array_element (Variables|Default|GetEffects)
    (Default|ApplyEffect _array_element (Variables|Default|GetOwnerHero))
    (if (<= (Variables|/Game/Core/Effects/BP_EffectBase.BP_EffectBase_C|GetEffectDuration _array_element) 0)
      (Utilities|Array|RemoveItem (Variables|Default|GetEffects) _array_element)
      (Actor|DestroyActor _array_element))))

(fn AddEffect
  (params (New%20effect :type BP%20Effect%20Base%20Object%20Reference))
  (Utilities|Array|AddUnique (Variables|Default|GetEffects) New%20effect))